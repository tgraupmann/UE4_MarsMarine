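; BP_MIssionAreaVolume is a volume that marks the mission area and punishes the player for leaving it.
; When a BP_Marine exits, it flags the marine as outside and starts a timer of SecondsBeforePlayerDeath; re-entering clears the flag and cancels the timer.
; On expiry, Kill Player applies 100 damage to player character 0, regardless of which marine left.
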(event `self.ReceiveActorBeginOverlap`
  (params (OtherActor :type "Actor Object Reference"))
  ;[1 1 1] Player Enters Mission Area
  (bind _asbp_marine (cast `/Game/Blueprints/Pawns/BP_Marine` OtherActor))
  (`Cpp_Marine.SetOutsideMissionArea` _asbp_marine false)
  (`KismetSystemLibrary.K2_ClearTimer` null "Kill Player"))

(event `self.ReceiveActorEndOverlap`
  (params (OtherActor :type "Actor Object Reference"))
  ;[1 1 1] Player Leaves Mission Area
  (bind _asbp_marine (cast `/Game/Blueprints/Pawns/BP_Marine` OtherActor))
  (`Cpp_Marine.SetOutsideMissionArea` _asbp_marine true)
  (`KismetSystemLibrary.K2_SetTimer` null "Kill Player" (`self.Seconds Before Player Death`)))

(fn `Kill Player`
  (`GameplayStatics.ApplyDamage` (`GameplayStatics.GetPlayerCharacter` 0) 100.0))

(fn `UserConstructionScript`)